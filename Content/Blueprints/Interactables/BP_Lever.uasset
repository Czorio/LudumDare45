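; BP_Lever is an interactable lever that switches a set of linked activatable objects on and off.
; Each interaction plays audio and toggles the HandleDown state, snapping the Handle between its rest rotation and a half-turn with no animation.
; It then calls Activate or Deactivate on every entry in the Activatable array to match the new state.
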(event `self.OnInteract`
  (params (Interactor :type "Pawn Object Reference"))
  (bind _activatable (`self.Activatable`))
  (`AudioComponent.Play` (`self.Audio`) 0.0)
  (if (`self.HandleDown`)
    (`SceneComponent.K2_SetRelativeRotation` :`self` (`self.Handle`))
    (set `self.HandleDown` false)
    (for _array_element _activatable
      (`/Game/Blueprints/Activatables/BP_Activatable.Deactivate` _array_element))
    (else
      (`SceneComponent.K2_SetRelativeRotation` (`self.Handle`) (struct :`Pitch` 180.0) false false)
      (set `self.HandleDown` true)
      (for _array_element_2 _activatable
        (`/Game/Blueprints/Activatables/BP_Activatable.Activate` _array_element_2)))))

(fn `UserConstructionScript`)