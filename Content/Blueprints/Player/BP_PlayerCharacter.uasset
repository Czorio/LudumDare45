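; BP_PlayerCharacter is the player character Blueprint, adding a reticule HUD and footstep audio.
; On BeginPlay it creates the WBP_Reticule widget for player 0 and adds it to the viewport.
; Tick checks the capsule's physics velocity, playing a 2D footstep cue on a timer while moving.
; When the character is still, the timer is set past the interval so the next movement triggers a step immediately.
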(event `self.ReceiveBeginPlay`
  (bind _returnvalue (`|CreateWidget` "/Game/UI/WBP_Reticule.WBP_Reticule_C" (`GameplayStatics.GetPlayerController` 0)))
  (`UserWidget.AddToViewport` _returnvalue 0))

(event `self.ReceiveTick`
  (params (DeltaSeconds :type "Float (single-precision)"))
  (bind _timesincelaststep (`self.TimeSinceLastStep`))
  (bind _returnvalue (`PrimitiveComponent.GetPhysicsLinearVelocity` (`self.CapsuleComponent`) "None"))
  (if (> (`KismetMathLibrary.VSize` _returnvalue) 1.0)
    (if (< _timesincelaststep (`self.TimeBetweenSteps`))
      (set `self.TimeSinceLastStep` (+ _timesincelaststep DeltaSeconds))
      (else
        (`GameplayStatics.SpawnSound2D` "/Game/Audio/Footstep_Cue.Footstep_Cue" 1.0 1.0 0.0 null)
        (set `self.TimeSinceLastStep` 0.0)))
    (else
      (set `self.TimeSinceLastStep` (+ (`self.TimeBetweenSteps`) 0.5)))))

(fn `UserConstructionScript`)