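; BP_OverheadLight is an activatable overhead light fixture with a light, an audio component and a static mesh.
; Activate shows the light, plays the audio and swaps the mesh's first material to an emissive version.
; Deactivate hides the light, stops the audio and sets the non-emissive material.
; The construction script only calls its parent.
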(event `self.Activate`
  (`SceneComponent.SetVisibility` (`self.Light`) true false)
  (`AudioComponent.Play` (`self.Audio`) 0.0)
  (`PrimitiveComponent.SetMaterial` (`self.StaticMesh`) 0 "/Game/Materials/M_OverheadLight_Emissive.M_OverheadLight_Emissive"))

(event `self.Deactivate`
  (`SceneComponent.SetVisibility` (`self.Light`) false false)
  (`AudioComponent.Stop` (`self.Audio`))
  (`PrimitiveComponent.SetMaterial` (`self.StaticMesh`) 0 "/Game/Materials/M_OverheadLight.M_OverheadLight"))

(fn `UserConstructionScript`
  (`parent.UserConstructionScript`))