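; Reactor activatable that runs the game's ending once activated.
; Activate runs a timed chain of delays: it lowers the Upper component, plays audio and then the reactor work cue.
; It then creates a player for EndSequence, reveals the Star's StarHot component, plays the sequence and quits the game after a fixed wait.
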(event `self.ReceiveBeginPlay`)

(event `self.Activate`
  (`KismetSystemLibrary.Delay` 1.0)
  (`SceneComponent.K2_SetRelativeLocation` (`self.Upper`) (0.0 0.0 -100.0) false false)
  (`AudioComponent.Play` (`self.Audio`) 0.0)
  (`KismetSystemLibrary.Delay` 2.0)
  (`AudioComponent.Play` (`self.ReactorWork_Cue`) 0.0)
  (`KismetSystemLibrary.Delay` 5.0)
  (bind _outactor (`LevelSequencePlayer.CreateLevelSequencePlayer` (`self.EndSequence`)))
  (`SceneComponent.SetVisibility` (`/Game/FXStarStarterKit/Blueprint/BP_HotStar.StarHot` (`self.Star`)) true true)
  (`MovieSceneSequencePlayer.Play` (`LevelSequenceActor.SequencePlayer` _outactor))
  (`KismetSystemLibrary.Delay` 26.0)
  (`KismetSystemLibrary.QuitGame` null "Quit"))

(fn `UserConstructionScript`
  (`parent.UserConstructionScript`))